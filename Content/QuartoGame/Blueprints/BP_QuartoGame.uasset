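; BP_QuartoGame is the Quarto game Blueprint, serving here as an on-screen debug readout of game state and current player.
; On BeginPlay it binds to the game-state-changed and current-player-changed events, caching each new value in a variable.
; Tick prints both cached enums as screen text every frame with zero duration, so they appear as a live display.
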(event `self.ReceiveBeginPlay`
  (add `self.OnGameStateChangedEvent` (delegate `OnGameStateChangedEvent_Event_0`))
  (add `self.OnCurrentPlayerChangedEvent` (delegate `OnCurrentPlayerChangedEvent_Event_0`)))

(event `OnCurrentPlayerChangedEvent_Event_0` :!signature `self.OnCurrentPlayerChangedEvent`
  (params (oldPlayer :type "EQuartoPlayer Enum" :default "Player_1") (newPlayer :type "EQuartoPlayer Enum" :default "Player_1"))
  (bind _output_get (set `self.d_currentPlayer` newPlayer)))

(event `OnGameStateChangedEvent_Event_0` :!signature `self.OnGameStateChangedEvent`
  (params (oldState :type "EQuartoGameState Enum" :default "GameStart") (newState :type "EQuartoGameState Enum" :default "GameStart"))
  (bind _output_get (set `self.d_gameState` newState)))

(event `self.ReceiveTick`
  (params (DeltaSeconds :type "Float (single-precision)"))
  (`KismetSystemLibrary.PrintString` (`KismetStringLibrary.Concat_StrStr` "Current game state: " (`|GetEnumeratorNameAsString` (stale `OnGameStateChangedEvent_Event_0` _output_get))) true false (struct :`G` 0.66 :`B` 1.0 :`A` 1.0) 0.0)
  (`KismetSystemLibrary.PrintString` (`KismetStringLibrary.Concat_StrStr` "Current player: " (`|GetEnumeratorNameAsString` (stale `OnCurrentPlayerChangedEvent_Event_0` _output_get))) true false (struct :`G` 0.66 :`B` 1.0 :`A` 1.0) 0.0))

(fn `UserConstructionScript`)